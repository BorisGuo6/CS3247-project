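; Player-held automatic weapon Blueprint that handles firing, reloading and recoil, using RU74 reload animations.
; A looping timer plays montages and spawns Bp_bullet at the muzzle socket, straight when aiming or randomly within a cone otherwise.
; Each shot consumes ammo and starts a timeline-driven recoil through controller pitch and yaw.
; Reload zeroes the magazine, plays empty or partial arm and weapon montages, then refills from reserve ammo on completion.
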(event `self.ReceiveBeginPlay`
  (bind _asplayer_bp (cast `/Game/Blueprints/Character/player_bp` (`GameplayStatics.GetPlayerPawn` 0)))
  (set `self.As Player Bp` _asplayer_bp))

(event `射击中`
  (bind (_return_value_location _returnvalue) (`self.子弹发射位置旋转`))
  (bind _as_player_anim (`/Game/Blueprints/Character/player_bp.As Player Anim` (`self.As Player Bp`)))
  (if (<= (`self.当前子弹数量`) 0)
    (`GameplayStatics.PlaySound2D` null 1.0 1.0 0.0 null null)
    (`KismetSystemLibrary.K2_ClearTimer` null "射击中")
    (else
      (`AnimInstance.Montage_Play` _as_player_anim (select `bool` (`/Game/Blueprints/Character/player_anim.是否瞄准` _as_player_anim) :!type "AnimMontage Object Reference") 1.2 "MontageLength" 0.0 true)
      (`AnimInstance.Montage_Play` (`SkeletalMeshComponent.GetAnimInstance` (`self.SkeletalMesh`)) null 2.5 "MontageLength" 0.0 true)
      (`|SpawnActorFromClass` "/Game/Blueprints/Weapon/bp_bullet.bp_bullet_C" (`KismetMathLibrary.MakeTransform` _return_value_location _returnvalue (0.2 0.2 0.2)) "AlwaysSpawn" "MultiplyWithRoot" null null)
      (bind _result (`/Engine/EditorBlueprintResources/StandardMacros.DecrementInt` (`self.当前子弹数量`))
        (:`  `
          (`KismetSystemLibrary.PrintString` (`KismetStringLibrary.Conv_IntToString` _result))
          (`self.后坐力计算`))))))

(event `开始射击`
  (`KismetSystemLibrary.K2_SetTimer` null "射击中" 0.12 true)
  (`self.射击中`))

(event `停止射击`
  (`KismetSystemLibrary.K2_ClearTimer` null "射击中"))

(event `开始换弹`
  (bind `_当前子弹数量` (`self.当前子弹数量`))
  (bind _returnvalue (<= (`self.子弹保存`) 0))
  (if (> (`self.总子弹数量`) 0)
    (if (not (== `_当前子弹数量` (`self.弹夹最大容量`)))
      (set `self.子弹保存` `_当前子弹数量`)
      (set `self.当前子弹数量` 0)
      (if (not (`self.正在换弹`))
        (set `self.正在换弹` true)
        (`|PlayMontage` (`Character.Mesh` (`self.As Player Bp`)) (select `bool` _returnvalue :`false` "/Game/FPS_Assault_Pack/Animations/RU74/A_Arms_RU74_Reload_Montage.A_Arms_RU74_Reload_Montage" :`true` "/Game/FPS_Assault_Pack/Animations/RU74/A_Arms_RU74_Reload_Empty_Montage.A_Arms_RU74_Reload_Empty_Montage" :!type "AnimMontage Object Reference")
          (:`then`
            (`|PlayMontage` (`self.SkeletalMesh`) (select `bool` _returnvalue :`false` "/Game/FPS_Assault_Pack/Animations/RU74/A_RU74_Reload_Montage.A_RU74_Reload_Montage" :`true` "/Game/FPS_Assault_Pack/Animations/RU74/A_RU74_Reload_Empty_Montage.A_RU74_Reload_Empty_Montage" :!type "AnimMontage Object Reference")
              (:`OnCompleted`
                (set `self.正在换弹` false)
                (`self.剩余子弹计算`)
                (bind _output_get (set `self.当前子弹数量` (`self.子弹保存`)))
                (`KismetSystemLibrary.PrintString` (`KismetStringLibrary.Conv_IntToString` _output_get) true true (struct :`R` 1.0 :`B` 0.071292 :`A` 1.0) 25.0)
                (`KismetSystemLibrary.PrintString` (`KismetStringLibrary.Conv_IntToString` (`self.总子弹数量`)) true true (struct :`G` 0.66 :`B` 1.0 :`A` 1.0) 25.0)))))))))

(event `后坐力计算`
  (bind _returnvalue (`GameplayStatics.GetPlayerPawn` 0))
  (bind (_direction `_新建轨道_0`) (`Timeline|时间轴` :!via `PlayFromStart`)
    (:`Update`
      (`Pawn.AddControllerYawInput` _returnvalue (`KismetMathLibrary.RandomFloatInRange` -0.1 0.1))
      (`Pawn.AddControllerPitchInput` _returnvalue (`KismetMathLibrary.Lerp` 0.0 -0.15 `_新建轨道_0`)))))

(fn `UserConstructionScript`)

(fn `剩余子弹计算`
  (bind _returnvalue (- (`self.总子弹数量`) (- (`self.弹夹最大容量`) (`self.子弹保存`))))
  (if (> _returnvalue 0)
    (set `self.总子弹数量` _returnvalue)
    (set `self.子弹保存` (`self.弹夹最大容量`))
    (else
      (set `self.子弹保存` (+ (`self.总子弹数量`) (`self.子弹保存`))))))

(fn `子弹发射位置旋转`
  (returns (`Return Value Location` :type "Vector Structure") (ReturnValue :type "Rotator Structure"))
  (bind (_returnvalue_location _returnvalue_rotation) (`KismetMathLibrary.BreakTransform` (`SceneComponent.GetSocketTransform` (`self.SkeletalMesh`) "b_Muzzle插槽" "RTS_World")))
  (return _returnvalue_location (select `bool` (`/Game/Blueprints/Character/player_anim.是否瞄准` (`/Game/Blueprints/Character/player_bp.As Player Anim` (`self.As Player Bp`))) :`false` (`KismetMathLibrary.Conv_VectorToRotator` (`KismetMathLibrary.RandomUnitVectorInConeInDegrees` (`KismetMathLibrary.Conv_RotatorToVector` _returnvalue_rotation) 5.0)) :`true` _returnvalue_rotation)))